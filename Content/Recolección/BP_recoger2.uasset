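; BP_recoger2 is a collectible pickup that adds a coin to the actor that touches it and then disappears.
; Four box components each handle begin overlap for one accepted class: recolectar_puntos, BP_tachometal, BP_cube or BP_tacho.
; On a successful cast, the handler calls that actor's SumarMoneda and destroys the pickup, ignoring other actors.
; A SetStaticMesh call on Sphera is left unconnected and never runs.
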(event `self.Box.OnComponentBeginOverlap`
  (params (OverlappedComponent :type "PrimitiveComponent Object Reference") (OtherActor :type "Actor Object Reference") (OtherComp :type "PrimitiveComponent Object Reference") (OtherBodyIndex :type Integer) (bFromSweep :type Boolean) (SweepResult :type "HitResult Structure (by ref)"))
  (bind _asrecolectar_puntos (cast `/Game/Recolección/recolectar_puntos` OtherActor))
  (`/Game/Recolección/recolectar_puntos.sumar moneda` _asrecolectar_puntos)
  (`self.K2_DestroyActor`))

(event `self.Box1.OnComponentBeginOverlap`
  (params (OverlappedComponent :type "PrimitiveComponent Object Reference") (OtherActor :type "Actor Object Reference") (OtherComp :type "PrimitiveComponent Object Reference") (OtherBodyIndex :type Integer) (bFromSweep :type Boolean) (SweepResult :type "HitResult Structure (by ref)"))
  (bind _asbp_tachometal (cast `/Game/Recolección/BP_tachometal` OtherActor))
  (`/Game/Recolección/BP_tachometal.sumar moneda` _asbp_tachometal)
  (`self.K2_DestroyActor`))

(event `self.Box2.OnComponentBeginOverlap`
  (params (OverlappedComponent :type "PrimitiveComponent Object Reference") (OtherActor :type "Actor Object Reference") (OtherComp :type "PrimitiveComponent Object Reference") (OtherBodyIndex :type Integer) (bFromSweep :type Boolean) (SweepResult :type "HitResult Structure (by ref)"))
  (bind _asbp_cube (cast `/Game/Recolección/BP_cube` OtherActor))
  (`/Game/Recolección/BP_cube.sumar moneda` _asbp_cube)
  (`self.K2_DestroyActor`))

(event `self.Box3.OnComponentBeginOverlap`
  (params (OverlappedComponent :type "PrimitiveComponent Object Reference") (OtherActor :type "Actor Object Reference") (OtherComp :type "PrimitiveComponent Object Reference") (OtherBodyIndex :type Integer) (bFromSweep :type Boolean) (SweepResult :type "HitResult Structure (by ref)"))
  (bind _asbp_tacho (cast `/Game/Recolección/BP_tacho` OtherActor))
  (`/Game/Recolección/BP_tacho.sumar moneda` _asbp_tacho)
  (`self.K2_DestroyActor`))

(fn `UserConstructionScript`)